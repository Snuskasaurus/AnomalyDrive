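; Configurable abandoned car prop, assembled from separate body, door, wheel, seat and trim meshes.
; The construction script pushes body color to the body, doors and fuel lid, and rust and dust values to most parts through material parameters.
; It rotates each door by its open and sagging values, mirroring the opening for the right side.
; Per-part booleans destroy unwanted components, allowing stripped-down variants from one Blueprint.
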(fn ConstructionScript
  (bind _staticmeshcomponent (Variables|Debug|GetStaticMeshComponent))
  ;[1 1 1] Body
  (Rendering|Material|SetVectorParameterValueonMaterials _staticmeshcomponent "color" (Math|Conversions|ToVector(LinearColor) (Math|Conversions|ToLinearColor(Color) (Variables|Body|GetColor))))
  (Rendering|Material|SetScalarParameterValueonMaterials _staticmeshcomponent "rust and wear" (Variables|Body|GetRust%20and%20wear))
  (Rendering|Material|SetScalarParameterValueonMaterials _staticmeshcomponent "dust" (Variables|Body|GetDust))
  ;[1 1 1] Doors Left
  (Transformation|AddLocalRotation (Variables|Default|GetSM_Door_FL) (Math|Rotator|MakeRotator (- 0.0 (Variables|Doors|GetDoor%20FL%20sagging)) 0.0 (Variables|Doors|GetDoor%20FL%20open)) false false)
  (Transformation|AddLocalRotation (Variables|Default|GetSM_Door_RL) (Math|Rotator|MakeRotator (- 0.0 (Variables|Doors|GetDoor%20RL%20sagging)) 0.0 (Variables|Doors|GetDoor%20RL%20open)) false false)
  ;[1 1 1] Doors Right
  (Transformation|AddLocalRotation (Variables|Default|GetSM_Door_FR) (Math|Rotator|MakeRotator (- 0.0 (Variables|Doors|GetDoor%20FR%20sagging)) 0.0 (- 0.0 (Variables|Doors|GetDoor%20FR%20open))) false false)
  (Transformation|AddLocalRotation (Variables|Default|GetSM_Door_RR) (Math|Rotator|MakeRotator (- 0.0 (Variables|Doors|GetDoor%20RR%20sagging)) 0.0 (- 0.0 (Variables|Doors|GetDoor%20RR%20open))) false false)
  ;[1 1 1] Doors hide
  (if (Variables|Doors|GetDoor%20FL)
    _
    (else
      (Components|DestroyComponent (Variables|Default|GetSM_Door_FL))))
  (if (Variables|Doors|GetDoor%20FR)
    _
    (else
      (Components|DestroyComponent (Variables|Default|GetSM_Door_FR))))
  (if (Variables|Doors|GetDoor%20RL)
    _
    (else
      (Components|DestroyComponent (Variables|Default|GetSM_Door_RL))))
  (if (Variables|Doors|GetDoor%20RR)
    _
    (else
      (Components|DestroyComponent (Variables|Default|GetSM_Door_RR))))
  ;[1 1 1] Elements hide
  (if (Variables|Details|GetSeat%20R)
    _
    (else
      (Components|DestroyComponent (Variables|Default|GetSM_Seat_R))))
  (if (Variables|Details|GetSeat%20L)
    _
    (else
      (Components|DestroyComponent (Variables|Default|GetSM_Seat_L))))
  (if (Variables|Details|GetFuel%20Lid)
    _
    (else
      (Components|DestroyComponent (Variables|Default|GetSM_Fuel_lid))))
  (if (Variables|Details|GetWheel%20FL)
    _
    (else
      (Components|DestroyComponent (Variables|Default|GetSM_Wheel2))))
  (if (Variables|Details|GetWheel%20FR)
    _
    (else
      (Components|DestroyComponent (Variables|Default|GetSM_Wheel1))))
  (if (Variables|Details|GetWheel%20RL)
    _
    (else
      (Components|DestroyComponent (Variables|Default|GetSM_Wheel4))))
  (if (Variables|Details|GetWheel%20RR)
    _
    (else
      (Components|DestroyComponent (Variables|Default|GetSM_Wheel3))))
  (if (Variables|Details|GetSuspension)
    _
    (else
      (Components|DestroyComponent (Variables|Default|GetSM_Suspension))))
  (if (Variables|Details|GetSteering%20Wheel)
    _
    (else
      (Components|DestroyComponent (Variables|Default|GetSM_Steering_Wheel))))
  (if (Variables|Details|GetExhaust)
    _
    (else
      (Components|DestroyComponent (Variables|Default|GetSM_Exhaust))))
  (if (Variables|Details|GetHeadlightR)
    _
    (else
      (Components|DestroyComponent (Variables|Default|GetSM_Headlight_R))))
  (if (not (Variables|Details|GetHeadlightL))
    (Components|DestroyComponent (Variables|Default|GetSM_Headlight_L))))