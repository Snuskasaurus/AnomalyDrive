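; ModularRoad is a road-building tool actor whose construction script rebuilds a road from socket-chained meshes or spline meshes.
; Mesh mode chains pieces at "F" sockets and can add seeded random buildings and socket labels; either mode can add an end spline to another road's socket.
; Helper functions edit and highlight pieces, snap to the nearest road socket, spawn roads at unreferenced sockets, and shape landscape along the end spline.
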(event EventBeginPlay)

(event Collision|EventActorBeginOverlap
  (params (OtherActor :type Actor%20Object%20Reference)))

(event EventTick
  (params (DeltaSeconds :type Float%20%28single-precision%29)))

(fn ConstructionScript
  (CallFunction|Construct))

(fn Add
  (params (Mesh :type Static%20Mesh%20Object%20Reference))
  (bind _mesharray (Variables|Editing|GetMeshArray))
  (Utilities|IsValid Mesh
    (:Is%20Valid
      (Utilities|Array|Add _mesharray Mesh))
    (:Is%20Not%20Valid
      (Utilities|Array|Add _mesharray (Utilities|Array|Get(acopy) _mesharray (Utilities|Array|LastIndex _mesharray)))))
  (CallFunction|Construct))

(fn Remove
  (params (Index :type Integer))
  (Utilities|Array|RemoveIndex (Variables|Editing|GetMeshArray) Index)
  (CallFunction|Construct))

(fn MakeEnds
  (bind _outactors (Actor|GetAllActorsOfClass "ModularRoad_C"))
  (Utilities|Array|RemoveItem _outactors self)
  (for _array_element _outactors
    (Utilities|IsValid (Variables|ModularRoad_C|GetSnapTarget _array_element)
      (:Is%20Valid
        (if (== (Variables|ModularRoad_C|GetSnapTarget _array_element) self)
          (Utilities|Array|Add (LocalVariables|GetIndexReferences) (Variables|ModularRoad_C|GetSnapTargetIndex _array_element))
          (Utilities|Array|Add (LocalVariables|GetSocketReferences) (Variables|ModularRoad_C|GetSnapTargetSocket _array_element))))))
  (for (_array_element_2 _array_index) (Variables|Save|GetAddedMeshes)
    (for _array_element_3 (Variables|Config|GetRoadSocketNames)
      (if (Transformation|DoesSocketExist _array_element_2 _array_element_3)
        (bind _referenced (|CheckIfReferenced _array_index _array_element_3))
        (if (not _referenced)
          (CallFunction|SpawnRoadatSocket _array_element_2 _array_index _array_element_3)
          (Math|Integer|IncrementInt (LocalVariables|GetCount))))))
  (Development|PrintString (Utilities|String|Append "Spawned " (Utilities|String|ToString(Integer) (LocalVariables|GetCount)) " New Roads!") true true "(R=0.000000,G=0.660000,B=1.000000,A=1.000000)" 5.0))

(fn SpawnRoadatSocket
  (params (Mesh :type Static%20Mesh%20Component%20Object%20Reference) (MeshIndex :type Integer) (SocketName :type Name))
  (Game|SpawnActorfromClass "ModularRoad_C" (Math|Transform|MakeTransform "0, 0, 0" "0, 0, 0" "1,1,1") "AlwaysSpawn" 0 0 0 true self MeshIndex SocketName false 0 0 "None" 0 0 0))

(fn DoSnaptoTarget
  (bind _snaptarget (Variables|Editing|GetSnapTarget))
  (bind _snaptargetindex (Variables|Editing|GetSnapTargetIndex))
  (bind _snaptargetsocket (Variables|Editing|GetSnapTargetSocket))
  (bind _addedmeshes (Variables|ModularRoad_C|GetAddedMeshes _snaptarget))
  (bind _output (Utilities|Array|Get(acopy) _addedmeshes _snaptargetindex))
  (bind _returnvalue (Transformation|GetSocketTransform _output _snaptargetsocket "RTS_World"))
  (bind (_roll _pitch _yaw) (Math|Rotator|BreakRotator (.rotation _returnvalue)))
  (if (Variables|Editing|GetSnapToTarget)
    (Utilities|IsValid _snaptarget
      (:Is%20Valid
        (Utilities|IsValid _output
          (:Is%20Valid
            (if (not (Utilities|Name|Equal(Name) _snaptargetsocket "None"))
              (Transformation|SetActorTransform (Math|Transform|MakeTransform (Class|KismetMathLibrary|VectorSnappedtoGrid (.location _returnvalue) 1.0) (Math|Rotator|MakeRotator (Math|Float|SnapToGrid(Float) _roll 1.0) (Math|Float|SnapToGrid(Float) _pitch 1.0) (Math|Float|SnapToGrid(Float) _yaw 1.0)) "1,1,1")))))))))

(fn Construct
  (bind _spline (Variables|Default|GetSpline))
  (CallFunction|Cleanup)
  (CallFunction|GenerateSeed)
  (Variables|Editing|SetNeedsRefresh false)
  (if (Variables|Editing|GetSplineMode)
    (if (> (Spline|GetNumberOfSplinePoints _spline) 1)
      (Spline|SetLocationatSplinePoint _spline 0 (Math|Vector|MakeVector 0.0 0.0 0.0) "Local" true)
      (Spline|SetTangentatSplinePoint _spline 0 (* "1.000000, 0, 0" (Math|Vector|VectorLength (Spline|GetTangentatSplinePoint _spline 0 "Local"))) "Local" true)
      (else
        (Spline|SetSplinePoints _spline (LocalVariables|GetDefaultSpline) "Local" true)
        (Spline|SetTangentatSplinePoint _spline 0 (Math|Vector|MakeVector 1e+04 0.0 0.0) "Local" true)))
    (CallFunction|MakeMeshforSpline _spline)
    (CallFunction|MakeEndSpline)
    (CallFunction|MakeMeshforSpline (Variables|Default|GetEndSpline))
    (else
      (Spline|SetSplinePoints (Variables|Default|GetSpline) (LocalVariables|GetEmptySpline) "Local" true)
      (CallFunction|MakeStaticMeshes)
      (CallFunction|MakeEndSpline)
      (CallFunction|MakeMeshforSpline (Variables|Default|GetEndSpline))
      (CallFunction|MakeBuildings)
      (CallFunction|DoEditMode)
      (if (and (not (Variables|Editing|GetSplineMode)) (not (Variables|Editing|GetMakeSplineEnd)))
        (if (== (Utilities|Array|LastIndex (Variables|Save|GetAddedMeshes)) -1)
          _
          (else
            (bind _array_element (Utilities|Array|ForEachLoopwithBreak (Variables|Save|GetAddedMeshes) :!label _label)
              (:LoopBody
                (Utilities|IsValid (Variables|/Script/Engine.StaticMeshComponent|GetStaticMesh _array_element)
                  (:Is%20Not%20Valid
                    (Utilities|FlowControl|Sequence
                      (:then_0
                        _)
                      (:then_1
                        (goto _label Break)))))))))
        ;[1 0 0] No Connected Paths
        (bind _returnvalue (AddComponent|AddStaticMeshComponent false (Math|Transform|MakeTransform "0, 0,1000.000000" "-90.000000, 0, 0" "20.000000,20.000000,20.000000")))
        (Components|StaticMesh|SetStaticMesh _returnvalue "/Engine/VREditor/TransformGizmo/TranslateArrowHandle.TranslateArrowHandle")
        (Rendering|Material|SetMaterial _returnvalue 1 "/Game/VOID_Game/Materials/Debug/Color_Red_Fullbright.Color_Red_Fullbright")
        (Utilities|Array|Add (Variables|Save|GetAddedMeshes) _returnvalue)))))

(fn MakeStaticMeshes
  (bind _addedmeshes (Variables|Save|GetAddedMeshes))
  ;[1 1 1] Cleanup
  (for _array_element (Variables|Save|GetAddedMeshes)
    (Utilities|IsValid _array_element
      (:Is%20Valid
        (Components|DestroyComponent _array_element))))
  (Utilities|Array|Clear (Variables|Save|GetAddedMeshes))
  ;[1 1 1] Create
  (for _array_element_2 (Variables|Editing|GetMeshArray)
    (bind _returnvalue (AddComponent|AddStaticMeshComponent false))
    (Components|StaticMesh|SetStaticMesh _returnvalue _array_element_2)
    (Utilities|Array|Add (Variables|Save|GetAddedMeshes) _returnvalue))
  ;[1 1 1] Place
  (for (_array_element_3 _array_index) _addedmeshes
    (if (> _array_index 0)
      (Transformation|SetWorldTransform _array_element_3 (Transformation|GetSocketTransform (Utilities|Array|Get(acopy) _addedmeshes (- _array_index 1)) "F" "RTS_World") false false))))

(fn DoEditMode
  (bind _addedtext (Variables|Save|GetAddedText))
  ;[1 1 1] Clear Existing
  (for _array_element _addedtext
    (Utilities|IsValid _array_element
      (:Is%20Valid
        (Components|DestroyComponent _array_element))))
  (Utilities|Array|Clear _addedtext)
  (if (Variables|Editing|GetEditMode)
    (for (_array_element_2 _array_index) (Variables|Save|GetAddedMeshes)
      (for _array_element_3 (Transformation|GetAllSocketNames _array_element_2)
        (if (Utilities|Array|ContainsItem (Variables|Config|GetRoadSocketNames) _array_element_3)
          (bind _returnvalue (AddComponent|AddTextRenderComponent false (Math|Transform|MakeTransform (+ (.Location (Math|Transform|BreakTransform (Transformation|GetSocketTransform _array_element_2 _array_element_3 "RTS_Actor"))) "0.000000, 0,100.000000" (* (Math|Vector|GetForwardVector (.Rotation (Math|Transform|BreakTransform (Transformation|GetSocketTransform _array_element_2 _array_element_3 "RTS_Actor")))) "-100.000000, 0, 0")) (Math|Rotator|CombineRotators (.Rotation (Math|Transform|BreakTransform (Transformation|GetSocketTransform _array_element_2 _array_element_3 "RTS_Actor"))) "0,180.000000, 0") "1,1,1")))
          (Rendering|Components|TextRender|SetText _returnvalue (Utilities|Text|ToText(String) (Utilities|String|Append (Utilities|String|ToString(Integer) _array_index) (Utilities|String|ToString(Name) _array_element_3))))
          (Utilities|Array|Add (Variables|Save|GetAddedText) _returnvalue))))))

(fn MakeEndSpline
  (bind _splineendtarget (Variables|Editing|GetSplineEndTarget))
  (bind _addedmeshes (Variables|Save|GetAddedMeshes))
  (bind _spline (Variables|Default|GetSpline))
  (bind _endtargetindex (Variables|Editing|GetEndTargetIndex))
  (bind _endtargetsocket (Variables|Editing|GetEndTargetSocket))
  (bind _returnvalue (Utilities|Array|LastIndex _addedmeshes))
  (bind _addedmeshes_2 (Variables|ModularRoad_C|GetAddedMeshes _splineendtarget))
  (bind _output (Utilities|Array|Get(acopy) _addedmeshes_2 _endtargetindex))
  (if (Variables|Editing|GetMakeSplineEnd)
    (Utilities|FlowControl|Sequence
      (:then_0
        ;[1 1 1] Create Spline Component
        (Utilities|IsValid (Variables|Default|GetEndSpline)
          (:Is%20Valid
            ;[1 1 1] Find End Location
            ;;[1 1 1] Check if Valid End Socket
            (Utilities|IsValid _output :!label _label
              (:Is%20Valid
                (if (Transformation|DoesSocketExist _output _endtargetsocket)
                  (LocalVariables|SetEndSocketTransform (|Rotate180 (Transformation|GetSocketTransform _output _endtargetsocket "RTS_World")))
                  (else
                    (LocalVariables|SetEndSocketTransform (Transformation|GetWorldTransform (Variables|ModularRoad_C|GetRoot (Variables|Editing|GetSplineEndTarget))))))
                ;[1 1 1] Set End Location and Tangent
                (Spline|SetLocationatSplinePoint (Variables|Default|GetEndSpline) 1 (.location (LocalVariables|GetEndSocketTransform)) "World" true)
                (Spline|SetTangentatSplinePoint (Variables|Default|GetEndSpline) 1 (* (Math|Rotator|GetRotationXVector (.rotation (LocalVariables|GetEndSocketTransform))) (Variables|Editing|GetSplineEndTangent)) "World" true)
                (Class|SplineComponent|SetUpVectoratSplinePoint (Variables|Default|GetEndSpline) 1 (Transformation|GetActorUpVector) "World" true))))
          (:Is%20Not%20Valid
            (bind _returnvalue_2 (AddComponent|AddSplineComponent false))
            (Variables|Default|SetEndSpline _returnvalue_2)
            ;[1 1 1] Set Start Location and Tangent
            (if (Variables|Editing|GetSplineMode)
              (LocalVariables|SetStartSocketTransform (Spline|GetTransformatSplinePoint _spline (- (Spline|GetNumberOfSplinePoints _spline) 1) "World" false))
              (elif (< _returnvalue 0)
                (LocalVariables|SetStartSocketTransform (Transformation|GetActorTransform))
                (else
                  (LocalVariables|SetStartSocketTransform (Transformation|GetSocketTransform (Utilities|Array|Get(acopy) _addedmeshes _returnvalue) "F" "RTS_World")))))
            (Spline|SetLocationatSplinePoint (Variables|Default|GetEndSpline) 0 (.location (LocalVariables|GetStartSocketTransform)) "World" true)
            (Spline|SetTangentatSplinePoint (Variables|Default|GetEndSpline) 0 (* (Math|Rotator|GetRotationXVector (.rotation (LocalVariables|GetStartSocketTransform))) (Variables|Editing|GetSplineEndTangent)) "World" true)
            (Class|SplineComponent|SetUpVectoratSplinePoint (Variables|Default|GetEndSpline) 0 (Transformation|GetActorUpVector) "World" true))))
      (:then_2
        (goto _label)))))

(fn MakeMeshforSpline
  (params (Spline :type Spline%20Component%20Object%20Reference))
  (bind _output_get (LocalVariables|SetInputSpline Spline))
  (Utilities|IsValid _output_get
    (:Is%20Valid
      (bind _output_get_2 (LocalVariables|SetSpacing (* (.X (Math|Vector|BreakVector (.BoxExtent (Math|BoxSphereBounds|BreakBoxSphereBounds (StaticMesh|GetBounds (Variables|Editing|GetSplineMesh)))))) 2.0)))
      (bind _output_get_3 (LocalVariables|SetLastIndex (.ReturnValue (Math|Float|Division(WholeandRemainder) (Spline|GetSplineLength (LocalVariables|GetInputSpline)) _output_get_2))))
      (for _index (range 0 _output_get_3)
        (LocalVariables|SetCurrentIndex _index)
        (bind _returnvalue (AddComponent|AddSplineMeshComponent false))
        (bind _output_get_4 (LocalVariables|SetSplineMeshRef _returnvalue))
        (Rendering|SetCastShadow _output_get_4 false)
        (Collision|SetCollisionEnabled _output_get_4 "QueryAndPhysics")
        (Components|StaticMesh|SetStaticMesh (LocalVariables|GetSplineMeshRef) (Variables|Editing|GetSplineMesh))
        (SplineMesh|SetStartandEnd (LocalVariables|GetSplineMeshRef) (Spline|GetLocationatDistanceAlongSpline (LocalVariables|GetInputSpline) (* (LocalVariables|GetCurrentIndex) (LocalVariables|GetSpacing)) "Local") (* (Spline|GetDirectionatDistanceAlongSpline (LocalVariables|GetInputSpline) (* (LocalVariables|GetCurrentIndex) (LocalVariables|GetSpacing)) "Local") (Math|Vector|Distance2D(Vector) (Spline|GetLocationatDistanceAlongSpline (LocalVariables|GetInputSpline) (* (LocalVariables|GetCurrentIndex) (LocalVariables|GetSpacing)) "Local") (Spline|GetLocationatDistanceAlongSpline (LocalVariables|GetInputSpline) (+ (* (LocalVariables|GetCurrentIndex) (LocalVariables|GetSpacing)) (LocalVariables|GetSpacing)) "Local"))) (Spline|GetLocationatDistanceAlongSpline (LocalVariables|GetInputSpline) (+ (* (LocalVariables|GetCurrentIndex) (LocalVariables|GetSpacing)) (LocalVariables|GetSpacing)) "Local") (* (Spline|GetDirectionatDistanceAlongSpline (LocalVariables|GetInputSpline) (+ (* (LocalVariables|GetCurrentIndex) (LocalVariables|GetSpacing)) (LocalVariables|GetSpacing)) "Local") (Math|Vector|Distance2D(Vector) (Spline|GetLocationatDistanceAlongSpline (LocalVariables|GetInputSpline) (* (LocalVariables|GetCurrentIndex) (LocalVariables|GetSpacing)) "Local") (Spline|GetLocationatDistanceAlongSpline (LocalVariables|GetInputSpline) (+ (* (LocalVariables|GetCurrentIndex) (LocalVariables|GetSpacing)) (LocalVariables|GetSpacing)) "Local"))) true :!class /Script/Engine.SplineMeshComponent)))))

(fn MakeBuildings
  (bind _addedbuildings (Variables|Save|GetAddedBuildings))
  (for _array_element _addedbuildings
    (Utilities|IsValid _array_element
      (:Is%20Valid
        (Components|DestroyComponent _array_element))))
  (Utilities|Array|Clear _addedbuildings)
  (if (Variables|Editing|GetAddBuildings)
    (for _array_element_2 (Variables|Save|GetAddedMeshes)
      (for _array_element_3 (Transformation|GetAllSocketNames _array_element_2)
        (if (or (Utilities|String|Contains (Utilities|String|ToString(Name) _array_element_3) "Mid") (Utilities|String|Contains (Utilities|String|ToString(Name) _array_element_3) "Corner"))
          (bind _returnvalue (AddComponent|AddStaticMeshComponent false))
          (Utilities|Array|Add (Variables|Save|GetAddedBuildings) _returnvalue)
          (Transformation|SetWorldLocationAndRotation _returnvalue (.location (Transformation|GetSocketTransform _array_element_2 _array_element_3 "RTS_World")) (.rotation (Transformation|GetSocketTransform _array_element_2 _array_element_3 "RTS_World")) false false)
          (if (Utilities|String|Contains (Utilities|String|ToString(Name) _array_element_3) "Mid")
            (Components|StaticMesh|SetStaticMesh _returnvalue (Utilities|GetRandomfromSeed (Variables|Config|GetBuildingsMid)))
            (elif (Utilities|String|Contains (Utilities|String|ToString(Name) _array_element_3) "Corner")
              (Components|StaticMesh|SetStaticMesh _returnvalue (Utilities|GetRandomfromSeed (Variables|Config|GetBuildingsCorner))))))))))

(fn SnaptoNearest
  (bind _outactors (Actor|GetAllActorsOfClass "ModularRoad_C"))
  (Utilities|Array|RemoveItem _outactors self)
  (for _array_element _outactors
    (for (_array_element_2 _array_index) (Variables|ModularRoad_C|GetAddedMeshes _array_element)
      (for _array_element_3 (Transformation|GetAllSocketNames _array_element_2)
        (if (not (Utilities|String|Contains (Utilities|String|ToString(Name) _array_element_3) "B_"))
          (bind _output_get (LocalVariables|SetCurrentDistance (Math|Vector|Distance2D(Vector) (Transformation|GetSocketLocation _array_element_2 _array_element_3) (Transformation|GetActorLocation))))
          (if (or (< _output_get (LocalVariables|GetBestDistance)) (== (LocalVariables|GetBestDistance) 0.0))
            (LocalVariables|SetBestDistance _output_get)
            (LocalVariables|SetBestSocketMeshIndex _array_index)
            (LocalVariables|SetBestSocketName _array_element_3)
            (LocalVariables|SetBestSocketOwner _array_element))))))
  (Variables|Editing|SetSnapTarget (LocalVariables|GetBestSocketOwner))
  (Variables|Editing|SetSnapTargetIndex (LocalVariables|GetBestSocketMeshIndex))
  (Variables|Editing|SetSnapTargetSocket (LocalVariables|GetBestSocketName))
  (Variables|Editing|SetSnapToTarget true)
  (CallFunction|DoSnaptoTarget)
  (Variables|Editing|SetNeedsRefresh true))

(fn Cleanup
  (bind _output_get (LocalVariables|SetMyChildren (Components|GetChildrenComponents (Variables|Default|GetRoot) false)))
  (for _array_element _output_get
    (Utilities|IsValid _array_element
      (:Is%20Valid
        (if (!= _array_element (Variables|Default|GetDefaultComponents))
          (Components|DestroyComponent _array_element)))))
  (Utilities|Array|Clear (Variables|Save|GetAddedMeshes))
  (Utilities|Array|Clear (Variables|Save|GetAddedText))
  (Utilities|Array|Clear (Variables|Save|GetAddedBuildings)))

(fn GetLastMeshIndex
  (return (Utilities|Array|LastIndex (Variables|Save|GetAddedMeshes))))

(fn GetSocketTransform
  (params (Index :type Integer) (SocketName :type Name))
  (return (Transformation|GetSocketTransform (Utilities|Array|Get(acopy) (Variables|Save|GetAddedMeshes) Index) SocketName "RTS_World")))

(fn HighlightIndex
  (params (Index :type Integer) (Color :type Linear%20Color%20Structure))
  (bind _returnvalue (Rendering|Material|CreateDynamicMaterialInstance "/Game/VOID_Game/Materials/Debug/Color_White_Fullbright.Color_White_Fullbright" "None" :!class /Script/Engine.KismetMaterialLibrary))
  (bind _output_get (LocalVariables|SetHighlightMaterial _returnvalue))
  (Rendering|Material|SetVectorParameterValue _output_get "Color" Color :!class /Script/Engine.MaterialInstanceDynamic)
  (for (_array_element _array_index) (Variables|Save|GetAddedMeshes)
    (if (== _array_index Index)
      (for _index (range 0 (Rendering|Material|GetNumMaterials _array_element))
        (Rendering|Material|SetMaterial _array_element _index (LocalVariables|GetHighlightMaterial)))
      (else
        (for _index_2 (range 0 (Rendering|Material|GetNumMaterials _array_element))
          (Rendering|Material|SetMaterial _array_element _index_2 0))))))

(fn ClearHighlights
  (for _array_element (Variables|Save|GetAddedMeshes)
    (for _index (range 0 (Rendering|Material|GetNumMaterials _array_element))
      (Rendering|Material|SetMaterial _array_element _index 0))))

(fn Replace
  (params (Index :type Integer) (Mesh :type Static%20Mesh%20Object%20Reference%20%28by%20ref%29))
  (Utilities|Array|SetArrayElem (Variables|Editing|GetMeshArray) Index Mesh true)
  (CallFunction|Construct))

(fn Insert
  (params (Index :type Integer) (Mesh :type Static%20Mesh%20Object%20Reference))
  (bind _mesharray (Variables|Editing|GetMeshArray))
  (Utilities|IsValid Mesh
    (:Is%20Valid
      (Utilities|Array|Insert _mesharray Mesh Index))
    (:Is%20Not%20Valid
      (Utilities|Array|Insert _mesharray (Utilities|Array|Get(acopy) _mesharray (Utilities|Array|LastIndex _mesharray)) Index)))
  (CallFunction|Construct))

(fn GenerateSeed
  (if (== (Variables|Editing|GetSeed) 0)
    (bind _output_get (Variables|Editing|SetSeed (Math|Random|RandomIntegerinRange 0 6464)))
    (Math|Random|SetRandomStreamSeed (Variables|Default|GetSeedStream) _output_get)
    (else
      (Math|Random|SetRandomStreamSeed (Variables|Default|GetSeedStream) (Variables|Editing|GetSeed)))))

(fn Landscape
  (bind _mylandscape (Variables|Config|GetMyLandscape))
  (bind _endspline (Variables|Default|GetEndSpline))
  (Utilities|IsValid _mylandscape
    (:Is%20Valid
      (Utilities|IsValid _endspline
        (:Is%20Valid
          (Landscape|Editor|EditorApplySpline _mylandscape _endspline 3e+03 3e+03 2e+03 2e+03 0.0 0.0 20 true true (Variables|Default|GetNewVar_0)))))))