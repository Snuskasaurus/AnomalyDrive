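; Spectator pawn for the vehicle system demo that shares its position over the network and lets the player leave spectating.
; While locally controlled, it passes its location to UpdateLocations every tick to store in WorldPos, with CamRot always zeroed.
; The WorldPos RepNotify teleports non-locally-controlled copies to that position.
; Q or End calls ExitSpectator on the VehiclePlayer controller.
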(event Custom|UpdateLocations
  (params (WorldPos :type Vector) (CamRot :type Rotator))
  (Variables|Default|SetWorldPos WorldPos)
  (Variables|Default|SetCamRot CamRot))

(event EventTick
  (params (DeltaSeconds :type Float%20%28single-precision%29))
  (if (Pawn|IsLocallyControlled)
    (CallFunction|UpdateLocations (Transformation|GetActorLocation) "0, 0, 0")))

(event Input|KeyboardEvents|End
  (params (Key :type Key%20Structure))
  (:Pressed
    (bind _asvehicle_player (Utilities|Casting|CastToVehiclePlayer (Pawn|GetController)))
    (Default|ExitSpectator _asvehicle_player)))

(event Input|KeyboardEvents|Q
  (params (Key :type Key%20Structure))
  (:Pressed
    (bind _asvehicle_player (Utilities|Casting|CastToVehiclePlayer (Pawn|GetController)))
    (Default|ExitSpectator _asvehicle_player)))

(fn ConstructionScript)

(fn OnRepWorldPos
  (if (not (Pawn|IsLocallyControlled))
    (Transformation|SetActorLocation (Variables|Default|GetWorldPos) false true)))