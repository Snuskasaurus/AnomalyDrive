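; Short-lived actor that displays a vehicle mesh as a red wireframe.
; The construction script assigns the VehicleMesh variable to its static mesh component, then overrides every material slot with Wireframe_Red.
; On BeginPlay it waits two seconds and destroys itself.
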(event EventBeginPlay
  (Utilities|FlowControl|Delay 2.0)
  (Actor|DestroyActor))

(fn ConstructionScript
  (bind _staticmesh (Variables|Default|GetStaticMesh))
  (Components|StaticMesh|SetStaticMesh _staticmesh (Variables|Default|GetVehicleMesh))
  (bind _output_get (LocalVariables|SetMats (Rendering|Material|GetMaterials _staticmesh)))
  (for (_ _array_index) _output_get
    (Rendering|Material|SetMaterial (Variables|Default|GetStaticMesh) _array_index "/Game/VehicleSystem/DemoAssets/Materials/Misc/Wireframe_Red.Wireframe_Red")))