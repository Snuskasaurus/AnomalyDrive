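; Player controller for the vehicle system demo that manages HUD, mouse input and spectator mode.
; It creates the demo HUD for the local player, toggles its sidebar with Q, and swaps in an autoshop HUD built per vehicle.
; Spectating possesses a spawned fast spectator; exiting teleports the stored character there and repossesses it.
; BeginPlay also runs a console command restoring vertical-FOV support on UE 4.26+.
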(event Custom|Display%20AutoShop%20HUD
  (params (Display :type Boolean) (Vehicle :type Vehicle%20Demo%20Base%20Object%20Reference))
  (bind _hud_autoshop (Variables|Default|GetHUD_AutoShop))
  ;[1 1 1] Autoshop
  (if (Pawn|IsLocalPlayerController)
    (Widget|SetVisibility (Variables|Default|GetHUD_Demo) (select Display "Hidden" "Visible"))
    (if Display
      (CallFunction|GenerateAutoshopHUD Vehicle)
      (CallFunction|SetMouseInputMode true)
      (else
        (CallFunction|ShowHUD true)
        (Utilities|IsValid _hud_autoshop
          (:Is%20Valid
            (Widget|RemovefromParent _hud_autoshop)))))))

(event Custom|ExitShop
  (params (Vehicle :type Vehicle%20Demo%20Base%20Object%20Reference))
  ;[1 1 1] Autoshop
  (Utilities|IsValid Vehicle
    (:Is%20Valid
      (Default|ExitAutoShop Vehicle))))

(event Custom|ShowHUD
  (params (Show :type Boolean))
  ;[1 1 1] Spectator Mode
  (if Show
    (Widget|SetVisibility (Variables|Default|GetHUD_Demo) "Visible")
    (CallFunction|SetMouseInputMode (Variables|/Game/VehicleSystem/DemoAssets/Blueprints/HUD/HUD_Demo.HUD_Demo_C|GetSidebarOpen (Variables|Default|GetHUD_Demo)))
    (else
      (Widget|SetVisibility (Variables|Default|GetHUD_Demo) "Hidden")
      (CallFunction|SetMouseInputMode false))))

(event Custom|ExitSpectator
  ;[1 1 1] Spectator Mode
  (bind _asspectator_fast (Utilities|Casting|CastToSpectatorFast (Pawn|GetControlledPawn)))
  (Variables|Default|SetSpectator _asspectator_fast)
  (Utilities|IsValid (Variables|Default|GetPlayerPawn)
    (:Is%20Valid
      (CallFunction|ShowHUD true)
      (bind _asdemo_character (Utilities|Casting|CastToDemoCharacter (Variables|Default|GetPlayerPawn)))
      (Transformation|Teleport _asdemo_character (Transformation|GetWorldLocation (Variables|/Script/Engine.DefaultPawn|GetCollisionComponent (Variables|Default|GetSpectator))) "0, 0, 0")
      (Pawn|Possess (Variables|Default|GetPlayerPawn))
      (Actor|DestroyActor (Variables|Default|GetSpectator)))))

(event Custom|SetMouseInputMode
  (params (bShowMouseCursor :type Boolean))
  (bind _self self)
  ;[1 1 1] MouseInput
  (bind _output_get (Variables|Default|SetbShowMouseCursor bShowMouseCursor))
  (if _output_get
    (Input|SetInputModeGameandUI _self 0 "DoNotLock" true)
    (else
      (Input|SetInputModeGameOnly _self))))

(event Custom|BecomeSpectator
  ;[1 1 1] Spectator Mode
  (bind _asdemo_character (Utilities|Casting|CastToDemoCharacter (Pawn|GetControlledPawn)))
  (Utilities|IsValid _asdemo_character
    (:Is%20Valid
      (Variables|Default|SetPlayerPawn _asdemo_character)
      (bind _returnvalue (Game|SpawnActorfromClass "/Game/VehicleSystem/DemoAssets/Blueprints/SpectatorFast.SpectatorFast_C" (Transformation|GetActorTransform _asdemo_character) "AlwaysSpawn" self 0))
      (bind _output_get (Variables|Default|SetSpectator _returnvalue))
      (Utilities|IsValid _output_get
        (:Is%20Valid
          (Pawn|Possess _output_get)
          (CallFunction|ShowHUD false)
          (bind _asdemo_character_2 (Utilities|Casting|CastToDemoCharacter (Variables|Default|GetPlayerPawn)))
          (Default|NetDisablePlayer _asdemo_character_2))))))

(event EventBeginPlay
  ;[0 0.7717 1] Init
  (if (Math|Boolean|ANDBoolean (Pawn|IsLocalPlayerController) (Variables|Default|GetCreateHUD) (not (Networking|IsDedicatedServer)))
    (bind _returnvalue (UserInterface|CreateWidget "/Game/VehicleSystem/DemoAssets/Blueprints/HUD/HUD_Demo.HUD_Demo_C" self))
    (bind _output_get (Variables|Default|SetHUD_Demo _returnvalue))
    (UserInterface|Viewport|AddtoViewport _output_get 0)
    (CallFunction|SetMouseInputMode false)
    (bind (_major _minor) (Class|VehicleSystemFunctions|GetUnrealEngineVersion))
    (if (or (== _major 5) (and (== _major 4) (>= _minor 26)))
      (Development|ExecuteConsoleCommand "r.UseLegacyMaintainYFOVViewMatrix 1" 0) ; Enables YFOV in UE4.26+, Epic disabled this\n and added this command as a cheat. Annoying the engine\ndoesn't really support this properly
    )))

(event EventDestroyed
  (bind _playerpawn (Variables|Default|GetPlayerPawn))
  (if (Networking|IsServer)
    (Utilities|IsValid _playerpawn
      (:Is%20Valid
        (Actor|DestroyActor _playerpawn)))))

(event EventPossess
  (params (PossessedPawn :type Pawn%20Object%20Reference))
  ;[0 0.7717 1] Init
  (|CallParentFunction PossessedPawn)
  (bind _asdemo_character (Utilities|Casting|CastToDemoCharacter PossessedPawn))
  (Variables|Default|SetPlayerPawn _asdemo_character))

(event Input|KeyboardEvents|Q
  (params (Key :type Key%20Structure :default "None"))
  (bind _hud_demo (Variables|Default|GetHUD_Demo))
  ;[1 1 1] Toggle Sidebar
  (:Pressed
    (Utilities|IsValid _hud_demo
      (:Is%20Valid
        (Default|ToggleSidebar _hud_demo)
        (CallFunction|SetMouseInputMode (Variables|/Game/VehicleSystem/DemoAssets/Blueprints/HUD/HUD_Demo.HUD_Demo_C|GetSidebarOpen (Variables|Default|GetHUD_Demo)))))))

(fn ConstructionScript)

(fn GenerateAutoshopHUD
  (params (Vehicle :type Vehicle%20Demo%20Base%20Object%20Reference))
  (bind _returnvalue (UserInterface|CreateWidget "/Game/VehicleSystem/DemoAssets/Blueprints/HUD/HUD_AutoShop.HUD_AutoShop_C" self))
  (bind _output_get (Variables|Default|SetHUD_AutoShop _returnvalue))
  (UserInterface|Viewport|AddtoViewport _output_get 0)
  (Default|ConstructforVehicle _output_get Vehicle))