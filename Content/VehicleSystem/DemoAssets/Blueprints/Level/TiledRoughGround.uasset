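; TiledRoughGround is a vehicle demo level actor that builds a tiled patch of ground from static mesh components.
; Its construction script runs a nested loop over SizeX and SizeY, adding one mesh per cell on a flat grid with 1000-unit spacing from the actor's origin.
; All layout happens at construction, and the event graph holds no active logic.
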(event EventBeginPlay)

(event Collision|EventActorBeginOverlap
  (params (OtherActor :type Actor%20Object%20Reference)))

(event EventTick
  (params (DeltaSeconds :type Float%20%28single-precision%29)))

(fn ConstructionScript
  (for _index (range 1 (Variables|Default|GetSizeX))
    (for _index_2 (range 1 (Variables|Default|GetSizeY))
      (AddComponent|AddStaticMeshComponent false (Math|Transform|MakeTransform (Math|Vector|MakeVector (Math|Conversions|ToFloat(Integer) (* (- _index 1) 1000)) (Math|Conversions|ToFloat(Integer) (* (- _index_2 1) 1000)) 0.0) "0, 0, 0" "1,1,1")))))