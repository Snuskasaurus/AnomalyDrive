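; Base vehicle Blueprint for a car that is assembled from installable parts.
; The construction script snaps a tagged Interactable box collider to each wheel, seat, engine and battery socket on the vehicle mesh.
; InstallCarPart records the part tag and spawns a static mesh on the matching socket, parenting wheels to their own wheel components and other parts to the body.
; Query functions report whether a part is installed or can still be installed.
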(event EventBeginPlay
  (|CallParentFunction))

(event EventTick
  (params (DeltaSeconds :type Float%20%28single-precision%29))
  (|CallParentFunction 0.0))

(event Custom|Install%20Car%20Part
  (params (CarPartTag :type Name) (Mesh :type Static%20Mesh%20Object%20Reference))
  (Utilities|Array|AddUnique (Variables|Default|GetInstalledCarPartTags) CarPartTag)
  (Components|CreateCarPartMesh CarPartTag Mesh))

(fn ConstructionScript
  (|CallParentFunction)
  (Components|CreateInteractableCollider "Wheel_FL")
  (Components|CreateInteractableCollider "Wheel_FR")
  (Components|CreateInteractableCollider "Wheel_BL")
  (Components|CreateInteractableCollider "Wheel_BR")
  (Components|CreateInteractableCollider "Seat_FL")
  (Components|CreateInteractableCollider "Seat_FR")
  (Components|CreateInteractableCollider "Seat_BL")
  (Components|CreateInteractableCollider "Seat_BR")
  (Components|CreateInteractableCollider "Engine")
  (Components|CreateInteractableCollider "Battery"))

(fn CreateInteractableCollider
  (params (CarPart :type Name))
  (bind _returnvalue (AddComponent|AddBoxComponent true))
  (bind _output_get (LocalVariables|SetCollider _returnvalue))
  (Variables|/Script/Engine.ActorComponent|SetComponentTags _output_get (Utilities|Array|MakeArray CarPart))
  (Components|Box|SetBoxExtent (LocalVariables|GetCollider) "10.000000,10.000000,10.000000" false)
  (Collision|SetCollisionProfileName (LocalVariables|GetCollider) "Interactable" false :!class /Script/Engine.PrimitiveComponent)
  (bind _returnvalue_2 (Transformation|AttachComponentToComponent (LocalVariables|GetCollider) (Variables|Default|GetVehicleMesh) CarPart "SnapToTarget" "SnapToTarget" "KeepWorld" true))
  (if (not _returnvalue_2)
    (Development|PrintString (Utilities|String|Append "Error: Failed to attach component on socket: (BP_Vehicle_Base::CreateInteractableCollider)" (Utilities|String|ToString(Name) CarPart)) true true "(R=1.000000,G=0.000000,B=0.001000,A=1.000000)" 1e+01)))

(fn CreateCarPartMesh
  (params (CarPart :type Name) (Mesh :type Static%20Mesh%20Object%20Reference))
  (bind _returnvalue (AddComponent|AddStaticMeshComponent true))
  (bind _output_get (LocalVariables|SetCarPartMesh _returnvalue))
  (bind _returnvalue_2 (Components|StaticMesh|SetStaticMesh _output_get Mesh))
  (if _returnvalue_2
    (Collision|SetCollisionProfileName (LocalVariables|GetCarPartMesh) "CarPart" false :!class /Script/Engine.PrimitiveComponent)
    (switch name CarPart
      (:Default
        _)
      (:Wheel_FL
        (LocalVariables|SetIndexMesh 1))
      (:Wheel_FR
        (LocalVariables|SetIndexMesh 2))
      (:Wheel_BL
        (LocalVariables|SetIndexMesh 3))
      (:Wheel_BR
        (LocalVariables|SetIndexMesh 4)))
    (bind _returnvalue_3 (Transformation|AttachComponentToComponent (LocalVariables|GetCarPartMesh) (Utilities|Select :Index (LocalVariables|GetIndexMesh) :Option%200 (Variables|Default|GetVehicleMesh) :Option%201 (Variables|Default|GetWheel_FL) :Option%202 (Variables|Default|GetWheel_FR) :Option%203 (Variables|Default|GetWheel_BL) :Option%204 (Variables|Default|GetWheel_BR)) CarPart "SnapToTarget" "SnapToTarget" "KeepWorld" true))
    (if (not _returnvalue_3)
      ;[0.15 0.15 0.15 0.5] Log Error
      (Development|PrintString (Utilities|String|Append "Error: Failed to attach component on socket: (BP_Vehicle_Base::CreateCarPart)" (Utilities|String|ToString(Name) CarPart)) true true "(R=1.000000,G=0.000000,B=0.001000,A=1.000000)" 1e+01))
    (else
      ;[0.15 0.15 0.15 0.5] Log Error
      (Development|PrintString (Utilities|String|Append "Error: Failed to set static mesh on socket: (BP_Vehicle_Base::CreateCarPart)" (Utilities|String|ToString(Name) CarPart)) true true "(R=1.000000,G=0.000000,B=0.001000,A=1.000000)" 1e+01))))

(fn CanInstalCarPart
  (params (CarPartTag :type Name%20%28by%20ref%29))
  (if (CarPart|IsCarPartInstalled CarPartTag)
    (return false)
    (else
      (return true))))

(fn IsCarPartInstalled
  (params (CarPartTag :type Name%20%28by%20ref%29))
  (return (Utilities|Array|ContainsItem (Variables|Default|GetInstalledCarPartTags) CarPartTag)))