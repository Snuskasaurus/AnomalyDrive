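; BP_CarPart is a car part actor with a physics-simulated static mesh that can be picked up.
; After a startup delay, Tick switches off simulation, mesh collision and ticking once linear and angular velocities drop below thresholds, saving cost.
; EnablePhysic reverses this, and both toggles print a debug message.
; OnPickup deactivates physics, hides the mesh and disables the Box collision; GetMeshToDisplay exposes the mesh, while GetCarpartInfo returns nothing.
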(event Custom|Enable%20Physic
  (Physics|SetSimulatePhysics (Variables|Default|GetStaticMesh) true)
  (Collision|SetCollisionEnabled (Variables|Default|GetStaticMesh) "PhysicsOnly")
  (Actor|Tick|SetActorTickEnabled true)
  ;[0.15 0.15 0.15 0.5] Comment
  (Development|PrintString (Utilities|String|Append "Activating Physic on " (Utilities|GetDisplayName self))))

(event Custom|Deactivate%20Physic
  (Physics|SetSimulatePhysics (Variables|Default|GetStaticMesh) false)
  (Collision|SetCollisionEnabled (Variables|Default|GetStaticMesh) "NoCollision")
  (Actor|Tick|SetActorTickEnabled false)
  ;[0.15 0.15 0.15 0.5] Comment
  (Development|PrintString (Utilities|String|Append "Deactivating Physic on " (Utilities|GetDisplayName self))))

(event Custom|On%20Pickup
  (CallFunction|DeactivatePhysic)
  (Development|SetHiddeninGame (Variables|Default|GetStaticMesh) true false)
  (Collision|SetCollisionEnabled (Variables|Default|GetBox) "NoCollision"))

(event EventTick
  (params (DeltaSeconds :type Float%20%28single-precision%29))
  (bind _staticmesh (Variables|Default|GetStaticMesh))
  (|CallParentFunction DeltaSeconds)
  (bind _output_get (Variables|Default|SetTimeSinceStart (+ (Variables|Default|GetTimeSinceStart) DeltaSeconds)))
  (if (>= _output_get (Variables|Default|GetTimeBeforeOptimization))
    (bind _returnvalue (Physics|GetPhysicsLinearVelocity _staticmesh "None"))
    (if (and (<= (Math|Vector|VectorLength _returnvalue) (Variables|Default|GetMinLinearVelocity)) (<= (Math|Vector|VectorLength (Physics|GetPhysicsAngularVelocityinDegrees _staticmesh "None")) (Variables|Default|GetMinAngularVelocity)))
      (CallFunction|DeactivatePhysic))))

(fn ConstructionScript)

(fn GetMeshtoDisplay
  (return (Variables|/Script/Engine.StaticMeshComponent|GetStaticMesh (Variables|Default|GetStaticMesh))))

(fn GetCarpartInfo
  (return ""))