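; BP_VehiclePart represents one part of a vehicle, identified by a part type and displayed through a static mesh.
; OnCreation stores the type, applies a default mesh, and hides the sprite and collision components in game.
; AddCarPart swaps in a supplied mesh, and IsInstalled treats a valid mesh as an installed part.
; RemoveCarPart is an empty stub.
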(event Custom|On%20Creation
  (params (CarPartType :type BPEnum_CarPartType%20Enum :default "NewEnumerator0") (DefaultMesh :type Static%20Mesh%20Object%20Reference))
  (Variables|Default|SetCarPartType CarPartType)
  (Components|StaticMesh|SetStaticMesh (Variables|Default|GetStaticMesh) DefaultMesh)
  (Development|SetHiddeninGame (Variables|Default|GetSpriteComponent) true false)
  (Development|SetHiddeninGame (Variables|Default|GetCollisionComponent) true false))

(fn ConstructionScript)

(fn IsInstalled
  (return (Utilities|IsValid (Variables|/Script/Engine.StaticMeshComponent|GetStaticMesh (Variables|Default|GetStaticMesh)))))

(fn RemoveCarPart)

(fn AddCarPart
  (params (StaticMeshFromPart :type Static%20Mesh%20Object%20Reference))
  (Components|StaticMesh|SetStaticMesh (Variables|Default|GetStaticMesh) StaticMeshFromPart))